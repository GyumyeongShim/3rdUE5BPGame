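; Main player controller for Gridventure that registers the game's input mapping and handles the grid inventory's input.
; The toggle action lazily creates WBP_Inventory, shows and refreshes it or removes it, and switches cursor, input mode and pause to match.
; The rotate action turns the dragged item's grid shape and drag visual, with a flag on the drag operation allowing one rotation per press.
; A ToggleInventory function duplicates the inline toggle logic.
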(event Input|EnhancedActionEvents|EnhancedInputActionIA_ToggleInventory
  (params (ActionValue :type Boolean) (ElapsedSeconds :type Float%20%28double-precision%29) (TriggeredSeconds :type Float%20%28double-precision%29) (InputAction :type Input%20Action%20Object%20Reference :default "/Game/Gridventure/Input/IA_ToggleInventory.IA_ToggleInventory"))
  (:Started
    (Utilities|IsValid (Variables|Default|GetInventoryWidget) ; 유효성 검사
      (:Is%20Valid
        _)
      (:Is%20Not%20Valid
        (bind _returnvalue (UserInterface|CreateWidget "/Game/Gridventure/Blueprints/UI/Inventory/WBP_Inventory.WBP_Inventory_C" self))
        (Variables|Default|SetInventoryWidget _returnvalue)))
    (if (UserInterface|Viewport|IsinViewport (Variables|Default|GetInventoryWidget))
      ;[0.15 0.15 0.15 0.5] 인벤토리 닫기
      (Widget|RemovefromParent (Variables|Default|GetInventoryWidget)) ; 인벤 닫기, 화면에서 제거
      (Variables|Default|SetbShowMouseCursor false)
      (Input|SetInputModeGameOnly self false) ; 마우스를 게임 월드 제어용으로 변경
      (Game|SetGamePaused false)
      (else
        ;[0.15 0.15 0.15 0.5] 인벤토리 열기
        (UserInterface|Viewport|AddtoViewport (Variables|Default|GetInventoryWidget) 0) ; 인벤 열기
        (Default|RefreshInventory (Variables|Default|GetInventoryWidget)) ; 시너지 스탯 적용 및 갱신
        (Variables|Default|SetbShowMouseCursor true)
        (Input|SetInputModeGameandUI self (Variables|Default|GetInventoryWidget) "DoNotLock" false false)
        (Game|SetGamePaused true) ; 게임 월드 정지
      ))))

(event Input|EnhancedActionEvents|EnhancedInputActionIA_InventoryRotateItem
  (params (ActionValue :type Boolean) (ElapsedSeconds :type Float%20%28double-precision%29) (TriggeredSeconds :type Float%20%28double-precision%29) (InputAction :type Input%20Action%20Object%20Reference :default "/Game/Gridventure/Input/IA_InventoryRotateItem.IA_InventoryRotateItem"))
  (bind _returnvalue (Class|WidgetBlueprintLibrary|GetDragDroppingContent))
  (bind _outputshape (|Rotateitem))
  (:Started
    (Utilities|IsValid _returnvalue
      (:Is%20Valid
        (bind _asbp_item_drag_op (Utilities|Casting|CastToBP_ItemDragOp _returnvalue))
        (Variables|Default|SetItemDragOp _asbp_item_drag_op)
        (if (Variables|/Game/Gridventure/Blueprints/UI/Inventory/BP_ItemDragOp.BP_ItemDragOp_C|GetbCanRoatate (Variables|Default|GetItemDragOp))
          (Utilities|Struct|SetmembersinF_ItemData (Variables|/Game/Gridventure/Blueprints/UI/Inventory/BP_ItemDragOp.BP_ItemDragOp_C|GetItemData (Variables|Default|GetItemDragOp)) _outputshape)
          (bind _aswbp_item_drag_visual (Utilities|Casting|CastToWBP_ItemDragVisual (Variables|/Script/UMG.DragDropOperation|GetDefaultDragVisual (Variables|Default|GetItemDragOp))))
          (Default|UpdateVisualShapeItem _aswbp_item_drag_visual _outputshape)
          (Default|UpdateVisualImageRotation _aswbp_item_drag_visual)
          (Variables|/Game/Gridventure/Blueprints/UI/Inventory/BP_ItemDragOp.BP_ItemDragOp_C|SetbCanRoatate (Variables|Default|GetItemDragOp) false)))))
  (:Completed
    (Variables|/Game/Gridventure/Blueprints/UI/Inventory/BP_ItemDragOp.BP_ItemDragOp_C|SetbCanRoatate (Variables|Default|GetItemDragOp) true)))

(event EventBeginPlay
  (Input|AddMappingContext (PlayerController|LocalPlayerSubsystems|GetEnhancedInputLocalPlayerSubsystem) "/Game/Gridventure/Input/IMC_MainGame.IMC_MainGame" 0 "(bIgnoreAllPressedKeysUntilRelease=True,bForceImmediately=False,bNotifyUserSettings=False)"))

(fn ConstructionScript)

(fn ToggleInventory
  (Utilities|IsValid (Variables|Default|GetInventoryWidget) ; 유효성 검사
    (:Is%20Valid
      _)
    (:Is%20Not%20Valid
      (bind _returnvalue (UserInterface|CreateWidget "/Game/Gridventure/Blueprints/UI/Inventory/WBP_Inventory.WBP_Inventory_C" self))
      (Variables|Default|SetInventoryWidget _returnvalue)))
  (if (UserInterface|Viewport|IsinViewport (Variables|Default|GetInventoryWidget))
    (Widget|RemovefromParent (Variables|Default|GetInventoryWidget)) ; 인벤 닫기, 화면에서 제거
    (Variables|Default|SetbShowMouseCursor false)
    (Input|SetInputModeGameOnly self false) ; 마우스를 게임 월드 제어용으로 변경
    (Game|SetGamePaused false)
    (else
      (UserInterface|Viewport|AddtoViewport (Variables|Default|GetInventoryWidget) 0) ; 인벤 열기
      (Default|RefreshInventory (Variables|Default|GetInventoryWidget)) ; 시너지 스탯 적용 및 갱신
      (Variables|Default|SetbShowMouseCursor true)
      (Input|SetInputModeGameandUI 0 (Variables|Default|GetInventoryWidget) "DoNotLock" false false)
      (Game|SetGamePaused true) ; 게임 월드 정지
    )))