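; Inventory component for a character that manages a grid of shaped items and drives weapon auto-attacks.
; Items occupy cells in a flattened width-by-height array, with helpers for space checks, placement, removal and rotation.
; Adjacency-based synergies accumulate stat bonuses and gameplay effect tags, which UpdateSynergy passes to the owning BP_BaseCharacter.
; ProcessAutoAtk gathers equipment with projectile classes, tracks per-ItemID cooldowns and requests projectiles at the nearest overlapping monster.
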(event EventBeginPlay
  (Utilities|Array|Resize (Variables|Default|GetInventoryArray) (* (Variables|Default|GetGridWidth) (Variables|Default|GetGridHeight)))
  ;[0.15 0.15 0.15 0.5] 테스트로 임시 Bullet
  (Utilities|Array|SetArrayElem (Variables|Default|GetInventoryArray) 0 (Utilities|Struct|MakeF_ItemData "Test_Staff" "" "(GameplayTags=((TagName=\"Item.Type.Equipment\")))" 0 0 "(MaxHp_12_E81349834A6504F2298A9A9601DA1109=0.000000,Atk_13_668D4F4F4DDDB0790A9817A621CBC3E2=0.000000,Def_14_B57BE2AF4B1581310E8F9285DAED9AE8=0.000000,Spd_15_2DBF5DEA4CC462C79B8814A7BC84F67D=0.000000,Accuracy_21_38D5DABA4721BF24A8B457A5666E4A40=0.000000,Evassion_20_B28FD9D64EE6A5D2DEDA66A0757E1E75=0.000000,CriChance_19_CC0BD56A4823B870A4B824926A984E0F=0.000000,Criresist_24_CF9263A24CABADBFA9FE3EB9EF66BD0D=0.000000)" 0 "" "/Game/Gridventure/Blueprints/Actor/BP_BaseProjectile.BP_BaseProjectile_C" 1.0 3e+02)))

(event EventTick
  (params (DeltaSeconds :type Float%20%28single-precision%29)))

(fn CheckSpace
  (params (StartPos :type Int%20Point%20Structure) (ItemData :type F%20Item%20Data%20Structure))
  (bind _gridshape (Utilities|Struct|BreakF_ItemData ItemData))
  (for (_ _array_index) _gridshape
    (if (Math|Boolean|ORBoolean (< (.X (Utilities|Struct|BreakIntPoint (+ StartPos (Utilities|Array|Get(acopy) _gridshape _array_index)))) 0) (< (.Y (Utilities|Struct|BreakIntPoint (+ StartPos (Utilities|Array|Get(acopy) _gridshape _array_index)))) 0) (>= (.X (Utilities|Struct|BreakIntPoint (+ StartPos (Utilities|Array|Get(acopy) _gridshape _array_index)))) (Variables|Default|GetGridWidth)) (>= (.Y (Utilities|Struct|BreakIntPoint (+ StartPos (Utilities|Array|Get(acopy) _gridshape _array_index)))) (Variables|Default|GetGridHeight)))
      (return false)
      (elif (== (.ItemID (Utilities|Struct|BreakF_ItemData (Utilities|Array|Get(acopy) (Variables|Default|GetInventoryArray) (+ (.X (Utilities|Struct|BreakIntPoint (+ StartPos (Utilities|Array|Get(acopy) _gridshape _array_index)))) (* (.Y (Utilities|Struct|BreakIntPoint (+ StartPos (Utilities|Array|Get(acopy) _gridshape _array_index)))) (Variables|Default|GetGridWidth)))))) "")
        (return true)
        (else
          (return false))))))

(fn AddItem
  (params (TopLeftPos :type Int%20Point%20Structure) (ItemData :type F%20Item%20Data%20Structure))
  ;[0.15 0.15 0.15 0.5] 슬롯 좌표, 인덱스 변환 (Y*Width + X)
  (for _array_element (.GridShape (Utilities|Struct|BreakF_ItemData ItemData))
    (Utilities|Array|SetArrayElem (Variables|Default|GetInventoryArray) (+ (.x (+ TopLeftPos _array_element)) (* (.y (+ TopLeftPos _array_element)) (Variables|Default|GetGridWidth))) ItemData))
  (Utilities|Array|Add (Variables|Default|GetPlacedItems) (Utilities|Struct|MakeF_PlacedItem ItemData TopLeftPos))
  (Default|CallOnInvenUpdated))

(fn RemoveItem
  (params (ItemData :type F%20Item%20Data%20Structure))
  (bind _placeditems (Variables|Default|GetPlacedItems))
  (bind _placeditems_2 (Variables|Default|GetPlacedItems))
  (bind _returnvalue (Utilities|Array|FindItem _placeditems_2 (Utilities|Struct|MakeF_PlacedItem ItemData "(X=0,Y=0)")))
  (bind _output (Utilities|Array|Get(acopy) _placeditems _returnvalue))
  (if (!= _returnvalue -1)
    (for _array_element (.gridshape (.itemdata _output))
      ;[0.15 0.15 0.15 0.5] 빈 데이터로 덮어쓰기
      (Utilities|Array|SetArrayElem (Variables|Default|GetInventoryArray) (+ (+ (.X (Utilities|Struct|BreakIntPoint _array_element)) (.x (.topleftpos _output))) (* (+ (.Y (Utilities|Struct|BreakIntPoint _array_element)) (.y (.topleftpos _output))) (Variables|Default|GetGridWidth))) (Utilities|Struct|MakeF_ItemData "None" "" "(GameplayTags=)" 0)))
    (Utilities|Array|RemoveIndex (Variables|Default|GetPlacedItems) _returnvalue)
    (Default|CallOnInvenUpdated)))

(fn RotateItem
  (params (InputShape :type Array%20of%20Int%20Point%20Structures))
  (for _array_element InputShape
    ;[0.15 0.15 0.15 0.5] 최소값 갱신
    (if (< (* (.Y (Utilities|Struct|BreakIntPoint _array_element)) -1) (LocalVariables|GetMinX))
      (LocalVariables|SetMinX (* (.Y (Utilities|Struct|BreakIntPoint _array_element)) -1))
      (if (< (.X (Utilities|Struct|BreakIntPoint _array_element)) (LocalVariables|GetMinY))
        (LocalVariables|SetMinY (.X (Utilities|Struct|BreakIntPoint _array_element)))
        (Utilities|Array|Add (LocalVariables|GetTempShpe) (Utilities|Struct|MakeIntPoint (LocalVariables|GetMinX) (LocalVariables|GetMinY))))))
  (return (LocalVariables|GetTempShpe) (LocalVariables|GetMinX) (LocalVariables|GetMinY)))

(fn RotateSinglePoint
  (params (IntputInt :type Vector%202D%20Structure) (MinX :type Integer) (MinY :type Integer))
  (bind (_x _y) (Math|Vector2D|BreakVector2D IntputInt))
  (return (Math|Vector2D|MakeVector2D (- (* _y -1.0) (* MinX 50)) (- _x (* MinY 50)))))

(fn CalcItemSynergy
  (params (TargetItemIdx :type Integer))
  (for _array_element (CallFunction|GetAdjacentIndicesbyShape)
    (if (!= (.ItemID (Utilities|Struct|BreakF_ItemData (Utilities|Array|Get(acopy) (Variables|Default|GetInventoryArray) _array_element))) "")
      (for _array_element_2 (.Synergy (Utilities|Struct|BreakF_ItemData (Utilities|Array|Get(acopy) (Variables|Default|GetInventoryArray) _array_element)))
        (if (GameplayTags|HasTag (.ItemType (Utilities|Struct|BreakF_ItemData (Utilities|Array|Get(acopy) (Variables|Default|GetInventoryArray) _array_element))) (.TargetTag (Utilities|Struct|BreakF_SynergyLogic _array_element_2)))
          (Math|Integer|IncrementInt (LocalVariables|GetFoundSynergyCnt)
            (:%20%20
              (GameplayTags|AddGameplayTag (LocalVariables|GetActiveEffects) (.EffectTag (Utilities|Struct|BreakF_SynergyLogic _array_element_2)) :!class /Script/GameplayTags.BlueprintGameplayTagLibrary)))))))
  (return (LocalVariables|GetActiveEffects) (LocalVariables|GetFoundSynergyCnt)))

(fn UpdateSynergy
  (Utilities|FlowControl|Sequence
    (:then_0
      ;[0.15 0.15 0.15 0.5] Init
      (Utilities|Array|Clear (LocalVariables|GetCheckedItemIDs))
      (Utilities|Array|Clear (LocalVariables|GetTotalBonusValue))
      (Utilities|Array|Resize (LocalVariables|GetTotalBonusValue) (|GetNumEnumEntries)))
    (:then_1
      (for (_array_element _array_index) (Variables|Default|GetInventoryArray)
        (if (and (!= (.ItemID (Utilities|Struct|BreakF_ItemData _array_element)) "") (not (Utilities|Array|ContainsItem (LocalVariables|GetCheckedItemIDs) (.ItemID (Utilities|Struct|BreakF_ItemData _array_element)))))
          (bind (_effecttag _foundsynergycnt) (CallFunction|CalcItemSynergy _array_index))
          (GameplayTags|AppendGameplayTagContainers (LocalVariables|GetAccumulatedEffects) _effecttag)
          (for (_array_element_2 _array_index_2) (.Synergy (Utilities|Struct|BreakF_ItemData _array_element))
            (Utilities|Array|SetArrayElem (LocalVariables|GetTotalBonusValue) _array_index_2 (+ (Utilities|Array|Get(acopy) (LocalVariables|GetTotalBonusValue) (Math|Conversions|ToInteger(Byte) (.stattoboost _array_element_2))) (* _foundsynergycnt (.bonusvalue _array_element_2))) true))))
      ;[0.15 0.15 0.15 0.5] 해당 캐릭터에게 시너지 적용
      (bind _asbp_base_character (Utilities|Casting|CastToBP_BaseCharacter (Components|GetOwner)))
      (Default|UpdateInvenSynergy _asbp_base_character (LocalVariables|GetTotalBonusValue) (LocalVariables|GetAccumulatedEffects)))
    (:then_2
      ;[0.15 0.15 0.15 0.5] 중복 방지를 위해 체크한 id를 추가
      (Utilities|Array|Add (LocalVariables|GetCheckedItemIDs) (.ItemID (Utilities|Struct|BreakF_ItemData _array_element))))))

(fn GetActiveWeapon
  (Utilities|Array|Clear (LocalVariables|GetActiveItems))
  (for _array_element (Variables|Default|GetInventoryArray)
    ;[0.15 0.15 0.15 0.5] Check Equipment Type
    (if (== (.ItemType (Utilities|Struct|BreakF_ItemData _array_element)) (GameplayTags|MakeGameplayTagContainerfromTag "(TagName=\"Item.Type.Equipment\")"))
      ;[0.15 0.15 0.15 0.5] Valid Projectile Class
      (if (Utilities|IsValidClass (.ProjectileClass (Utilities|Struct|BreakF_ItemData _array_element)))
        (Utilities|Array|Add (LocalVariables|GetActiveItems) _array_element))))
  (return (LocalVariables|GetActiveItems)))

(fn ProcessAutoAtk
  (bind _activeitemarray (CallFunction|GetActiveWeapon))
  (for _array_element _activeitemarray
    (if (.ReturnValue (Utilities|Map|Find (Variables|Default|GetWeaponCooldownMap) (.itemid _array_element)))
      (if (>= (- (Utilities|Time|GetGameTimeinSeconds) (.Value (Utilities|Map|Find (Variables|Default|GetWeaponCooldownMap) (.itemid _array_element)))) (.firerate _array_element))
        ;[0.15 0.15 0.15 0.5] 타겟 탐색
        (bind _targetactor (CallFunction|GetNearestEnemy (.range _array_element) :!label _label))
        (Utilities|IsValid _targetactor
          (:Is%20Valid
            ;[0.15 0.15 0.15 0.5] 투사체 생성
            (bind _asbp_base_character (Utilities|Casting|CastToBP_BaseCharacter (Components|GetOwner)))
            (Default|RequestSpawnProjectile _asbp_base_character (.projectileclass _array_element) _targetactor)
            ;[0.15 0.15 0.15 0.5] 발사 시간 누적
            (Utilities|Map|Add (Variables|Default|GetWeaponCooldownMap) (.itemid _array_element) (Utilities|Time|GetGameTimeinSeconds)))))
      (else
        (goto _label)))))

(fn GetNearestEnemy
  (params (Radius :type Float%20%28double-precision%29))
  (bind _returnvalue (Components|GetOwner))
  (bind _outactors (Collision|SphereOverlapActors (Transformation|GetActorLocation _returnvalue) Radius (Utilities|Array|MakeArray "ObjectTypeQuery3") "/Game/Gridventure/Blueprints/Actor/BP_BaseMonster.BP_BaseMonster_C"))
  (for _array_element _outactors
    (if (< (Transformation|GetDistanceTo _array_element _returnvalue) (LocalVariables|GetMinDist))
      (LocalVariables|SetMinDist (Transformation|GetDistanceTo _array_element _returnvalue))
      (LocalVariables|SetClosestTarget _array_element)))
  (return (LocalVariables|GetClosestTarget)))