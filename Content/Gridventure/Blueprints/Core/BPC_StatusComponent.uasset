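; Actor component that applies Fire, Poison and Lightning statuses as timed damage-over-time on its owner, driven by DT_StatusData rows.
; ApplyStatusEffect routes tags to ExecuteStatusEffect, which starts looping tick timers tracked per tag and ended by one RetriggerableDelay.
; On expiry, HandleSpecialLogic is meant to chain statuses to nearby pawns' components via sphere overlap.
; That call passes zero range and chain count, so spreading never runs.
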(event Custom|OnStatusTick
  (bind _returnvalue (Utilities|GetDataTableRow "/Game/Gridventure/Blueprints/Data/DataTable/DT_StatusData.DT_StatusData" (GameplayTags|GetTagName (stale Custom|AddandSetDelay Status)))
    (:then
      (Game|Damage|ApplyDamage (Components|GetOwner) (.Dot (Utilities|Struct|BreakF_StatusData _returnvalue)) 0 0))))

(event Custom|AddandSetDelay
  (params (Status :type Gameplay%20Tag%20Structure) (Duration :type Float%20%28double-precision%29) (TickInterval :type Float%20%28double-precision%29) (bHasSpecialEffect :type Boolean) (ChainCnt :type Integer))
  (bind _returnvalue (Utilities|Time|SetTimerbyEvent (delegate Custom|OnStatusTick) TickInterval true))
  (Utilities|Map|Add (Variables|Default|GetActiveStatusTimers) Status _returnvalue)
  (Utilities|FlowControl|RetriggerableDelay Duration)
  (Utilities|Time|ClearandInvalidateTimerbyHandle _returnvalue)
  (Utilities|Map|Remove (Variables|Default|GetActiveStatusTimers) Status)
  (if bHasSpecialEffect
    (CallFunction|HandleSpecialLogic)))

(fn ApplyStatusEffect
  (params (StatusEffectTag :type Gameplay%20Tag%20Container%20Structure) (ChainCnt :type Integer))
  (Utilities|IsValid (Actor|GetComponentbyClass (Components|GetOwner) "BPC_StatusComponent_C")
    (:Is%20Valid
      (for _array_element (GameplayTags|BreakGameplayTagContainer StatusEffectTag)
        (if (.ReturnValue (Utilities|Map|Find (Variables|Default|GetActiveStatusTimers) _array_element))
          (CallFunction|ExecuteStatusEffect _array_element) ; 상태이상 보유한 경우
          (else
            (|SwitchGameplayTag _array_element ; 새로 획득하는 경우
              (:Attribute.Fire
                (CallFunction|ExecuteStatusEffect _array_element :!label _label))
              (:Attribute.Lightning
                (if (not (> ChainCnt 0))
                  (bind _returnvalue (Utilities|GetDataTableRow "/Game/Gridventure/Blueprints/Data/DataTable/DT_StatusData.DT_StatusData" (GameplayTags|GetTagName _array_element)) ; 전이효과 최초 발생인 경우 진행
                    (:then
                      (bind _output_get (LocalVariables|SetLocal_ChainCnt (.MaxChainCnt (Utilities|Struct|BreakF_StatusData _returnvalue))))
                      (CallFunction|ExecuteStatusEffect _array_element _output_get)))))
              (:Attribute.Poison
                (goto _label)))))))))

(fn ExecuteStatusEffect
  (params (StatusTag :type Gameplay%20Tag%20Structure) (ChainCnt :type Integer))
  (bind _activestatustimers (Variables|Default|GetActiveStatusTimers))
  (bind (_value _returnvalue) (Utilities|Map|Find _activestatustimers StatusTag))
  (bind _returnvalue_2 (Utilities|GetDataTableRow "/Game/Gridventure/Blueprints/Data/DataTable/DT_StatusData.DT_StatusData" (GameplayTags|GetTagName StatusTag))
    (:then
      (if _returnvalue
        (Utilities|Time|ClearandInvalidateTimerbyHandle _value))
      (CallFunction|AddandSetDelay (.StatusTag (Utilities|Struct|BreakF_StatusData _returnvalue_2)) (.Duration (Utilities|Struct|BreakF_StatusData _returnvalue_2)) (.TickInterval (Utilities|Struct|BreakF_StatusData _returnvalue_2)) (.bHasSpecialEffect (Utilities|Struct|BreakF_StatusData _returnvalue_2)) ChainCnt))))

(fn HandleSpecialLogic
  (params (StatusTag :type Gameplay%20Tag%20Structure) (SpecialRange :type Float%20%28double-precision%29) (ChainCnt :type Integer))
  (Utilities|IsValid (Actor|GetComponentbyClass (Components|GetOwner) "BPC_StatusComponent_C")
    (:Is%20Valid
      (if (not (Utilities|Map|Contains (Variables|Default|GetActiveStatusTimers) StatusTag)) ; 중복 상태 이상 체크 (이미 있다면 넘어가기)
        (if (> ChainCnt 0) ; 체인 차감
          (bind _outactors (Collision|SphereOverlapActors (Transformation|GetActorLocation (Components|GetOwner)) SpecialRange (Utilities|Array|MakeArray "ObjectTypeQuery3") 0 (Utilities|Array|MakeArray (Components|GetOwner))))
          (for _array_element _outactors
            (if (!= _array_element (Components|GetOwner))
              (bind _output_get (LocalVariables|Setcnt (- ChainCnt 1)))
              (CallFunction|ApplyStatusEffect (Actor|GetComponentbyClass _array_element "BPC_StatusComponent_C") (GameplayTags|MakeGameplayTagContainerfromArray (Utilities|Array|MakeArray StatusTag)) _output_get))))))))