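; Actor component that holds a unit's base stats, current HP, experience and level.
; BeginPlay fills HP to max, and TakeDmg subtracts GetFinalDmg from attack, defense and skill power, destroying the owner at zero HP.
; AddExp only accumulates experience, as its LevelUp call is disconnected.
; LevelUp increments the level, resets experience and rebuilds the stat struct with higher max HP, attack and defense.
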(event EventBeginPlay
  (Variables|Default|SetCurHp (.MaxHp (Utilities|Struct|BreakF_StatData (Variables|Default|GetBaseStat)))))

(event EventTick
  (params (DeltaSeconds :type Float%20%28single-precision%29)))

(fn TakeDmg
  (params (AtkerAtk :type Float%20%28double-precision%29) (SkillPower :type Float%20%28double-precision%29))
  ;[0.15 0.15 0.15 0.5] if (CurHP <= 0)
  (bind _output_get (Variables|Default|SetCurHp (Math|Float|Max(Float) (- (Variables|Default|GetCurHp) (CallFunction|GetFinalDmg AtkerAtk (.Def (Utilities|Struct|BreakF_StatData (Variables|Default|GetBaseStat))) SkillPower)) 0.0)))
  (if (<= _output_get 0.0)
    (Actor|DestroyActor (Components|GetOwner))))

(fn AddExp
  (params (Exp :type Float%20%28double-precision%29))
  ;[0.15 0.15 0.15 0.5] 경험치 획득
  (Variables|Default|SetCurExp (+ Exp (Variables|Default|GetCurExp))))

(fn LevelUp
  (Variables|Default|SetCurLevel (+ (Variables|Default|GetCurLevel) 1))
  (Variables|Default|SetCurExp 0.0)
  (Variables|Default|SetBaseStat (Utilities|Struct|MakeF_StatData (+ (.MaxHp (Utilities|Struct|BreakF_StatData (Variables|Default|GetBaseStat))) 2e+01) (+ (.Atk (Utilities|Struct|BreakF_StatData (Variables|Default|GetBaseStat))) 2.0) (+ (.Def (Utilities|Struct|BreakF_StatData (Variables|Default|GetBaseStat))) 1.0) (.Spd (Utilities|Struct|BreakF_StatData (Variables|Default|GetBaseStat))) (.Accuracy (Utilities|Struct|BreakF_StatData (Variables|Default|GetBaseStat))) (.Evassion (Utilities|Struct|BreakF_StatData (Variables|Default|GetBaseStat))) (.CriChance (Utilities|Struct|BreakF_StatData (Variables|Default|GetBaseStat))) (.Criresist (Utilities|Struct|BreakF_StatData (Variables|Default|GetBaseStat))))))