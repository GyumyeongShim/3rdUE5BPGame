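; Base character Blueprint for Gridventure, handling input movement, montage melee attacks, damage intake and projectile spawning.
; Attacks switch Locomotion to Battle, and a weapon-socket sphere trace damages "Monster" actors through their stat component using base Atk.
; Incoming damage reaches its own stat component, followed by brief invincibility.
; Inventory synergy bonuses combine with base stats into FinalStatData, adding Spd onto current walk speed each refresh.
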(event Custom|AtkEnd
  ;[0.15 0.15 0.15 0.5] 공격 종료시 호출
  (Variables|Default|SetState "NewEnumerator0"))

(event Custom|OnAtkHitEnd)

(event Custom|OnAtkHitStart
  (bind _mesh (Variables|Character|GetMesh))
  (bind _outhit (Collision|SphereTraceByChannel (Transformation|GetSocketLocation _mesh "TrailStart") (Transformation|GetSocketLocation _mesh "TrailEnd") 5e+01 "TraceTypeQuery1" false 0 "ForDuration"))
  ;[0.15 0.15 0.15 0.5] Tag 유효성 체크
  (if (Actor|ActorHasTag (.HitActor (Collision|BreakHitResult _outhit)) "Monster")
    ;[0.15 0.15 0.15 0.5] StatComponent 유효성
    (if (Utilities|IsValid (Actor|GetComponentbyClass (.HitActor (Collision|BreakHitResult _outhit)) "/Game/Gridventure/Blueprints/Core/BPC_StatComponent.BPC_StatComponent_C"))
      ;[0.15 0.15 0.15 0.5] Dmg 처리
      (Default|TakeDmg (Actor|GetComponentbyClass (.HitActor (Collision|BreakHitResult _outhit)) "/Game/Gridventure/Blueprints/Core/BPC_StatComponent.BPC_StatComponent_C") self (.atk (Variables|/Game/Gridventure/Blueprints/Core/BPC_StatComponent.BPC_StatComponent_C|GetBaseStat (Variables|Default|GetBPC_StatComponent))) 1e+02))))

(event Input|EnhancedActionEvents|EnhancedInputActionIA_Move
  (params (ActionValue :type Vector%202D%20Structure) (ElapsedSeconds :type Float%20%28double-precision%29) (TriggeredSeconds :type Float%20%28double-precision%29) (InputAction :type Input%20Action%20Object%20Reference :default "/Game/Gridventure/Input/IA_Move.IA_Move"))
  ;[0.15 0.15 0.15 0.5] 이동 키 입력 처리
  (Pawn|Input|AddMovementInput (Math|Vector|GetForwardVector (Pawn|GetControlRotation :!class /Script/Engine.Pawn)) (.y ActionValue) false)
  (Pawn|Input|AddMovementInput (Math|Vector|GetRightVector (Pawn|GetControlRotation :!class /Script/Engine.Pawn)) (.x ActionValue) false))

(event Input|EnhancedActionEvents|EnhancedInputActionIA_Atk
  (params (ActionValue :type Boolean) (ElapsedSeconds :type Float%20%28double-precision%29) (TriggeredSeconds :type Float%20%28double-precision%29) (InputAction :type Input%20Action%20Object%20Reference :default "/Game/Gridventure/Input/IA_Atk.IA_Atk"))
  ;[0.15 0.15 0.15 0.5] 공격 키 입력에 따른 state 변경, montage 변경
  (:Triggered
    (switch Utilities|FlowControl|Switch|SwitchonEPlayerState (Variables|Default|GetState) :!label _label
      (:NewEnumerator0
        (Variables|Default|SetState "NewEnumerator2")
        (Animation|PlayAnimMontage "/Game/Gridventure/Blueprints/Actor/AM_Atk.AM_Atk" 1.0 "None"))))
  (:Started
    (goto _label)))

(event Game|Damage|EventAnyDamage
  (params (Damage :type Float%20%28single-precision%29) (DamageType :type Damage%20Type%20Object%20Reference) (InstigatedBy :type Controller%20Object%20Reference) (DamageCauser :type Actor%20Object%20Reference))
  ;[0.15 0.15 0.15 0.5] 데미지 전달
  (if (not (Variables|Default|GetIsInvincible))
    (Default|TakeDmg (Variables|Default|GetBPC_StatComponent) self Damage 1e+02)
    (Variables|Default|SetIsInvincible true)
    (Utilities|FlowControl|RetriggerableDelay 0.5)
    (Variables|Default|SetIsInvincible false)))

(fn ConstructionScript)

(fn UpdateInvenSynergy
  (params (NewBonusArray :type Array%20of%20Floats%20%28double-precision%29) (NewEffectTags :type Gameplay%20Tag%20Container%20Structure))
  (Variables|Default|SetSynergyBonusArray NewBonusArray)
  (Variables|Default|SetSynergyTag NewEffectTags)
  (CallFunction|RefreshFinalStat))

(fn RefreshFinalStat
  (bind _charactermovement (Variables|Character|GetCharacterMovement))
  (bind _bpc_statcomponent (Variables|Default|GetBPC_StatComponent))
  (bind _finalstatvalue (LocalVariables|GetFinalStatValue))
  (bind _basestat (Variables|/Game/Gridventure/Blueprints/Core/BPC_StatComponent.BPC_StatComponent_C|GetBaseStat _bpc_statcomponent))
  (bind (_maxhp _atk _def _spd _accuracy _evassion _crichance _criresist) (Utilities|Struct|BreakF_StatData _basestat))
  (Utilities|Array|Resize (LocalVariables|GetFinalStatValue) (|GetNumEnumEntries))
  ;[0.15 0.15 0.15 0.5] Stat Data + Synergy Bonus Array = > Final Stat Value
  (for (_array_element _array_index) (Variables|Default|GetSynergyBonusArray)
    (Utilities|Array|SetArrayElem (LocalVariables|GetFinalStatValue) _array_index (+ _array_element (Utilities|Select :Index _array_index :Option%200 _maxhp :Option%201 _atk :Option%202 _def :Option%203 _spd :Option%204 _accuracy :Option%205 _evassion :Option%206 _crichance :Option%207 _criresist))))
  ;[0.15 0.15 0.15 0.5] Result
  (bind _output_get (Variables|Default|SetFinalStatData (Utilities|Struct|MakeF_StatData (Utilities|Array|Get(acopy) _finalstatvalue) (Utilities|Array|Get(acopy) _finalstatvalue 1) (Utilities|Array|Get(acopy) _finalstatvalue 2) (Utilities|Array|Get(acopy) _finalstatvalue 3) (Utilities|Array|Get(acopy) _finalstatvalue 4) (Utilities|Array|Get(acopy) _finalstatvalue 5) (Utilities|Array|Get(acopy) _finalstatvalue 6) (Utilities|Array|Get(acopy) _finalstatvalue 7))))
  ;[0.15 0.15 0.15 0.5] Max walk spd + spd => Max Walk Spd
  (Variables|/Script/Engine.CharacterMovementComponent|SetMaxWalkSpeed _charactermovement (+ (Variables|/Script/Engine.CharacterMovementComponent|GetMaxWalkSpeed _charactermovement) (.Spd (Utilities|Struct|BreakF_StatData _output_get))))
  (Default|CallOnStatUpdated))

(fn RequestSpawnProjectile
  (params (ProjectileClass :type Actor%20Class%20Reference) (TargetActor :type Actor%20Object%20Reference))
  (bind _returnvalue (Transformation|GetActorLocation))
  (bind _returnvalue_2 (+ (.z _returnvalue) 7e+01))
  (bind _returnvalue_3 (Math|Vector|MakeVector (.x _returnvalue) (.y _returnvalue) _returnvalue_2))
  (Game|SpawnActorfromClass ProjectileClass (Math|Transform|MakeTransform _returnvalue_3 (Math|Rotator|FindLookatRotation _returnvalue_3 (Transformation|GetActorLocation TargetActor))) "AlwaysSpawn" "MultiplyWithRoot" 0 0))