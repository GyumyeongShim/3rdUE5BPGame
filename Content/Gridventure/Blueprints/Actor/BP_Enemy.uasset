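; BP_Enemy is an enemy actor that deals and receives damage through stat components.
; AnyDamage forwards incoming damage to its own stat component, passing itself as the attacker.
; At attack hit start, a single debug-drawn sphere trace between the mesh's trail sockets damages a hit actor's stat component using the enemy's base attack.
; Other events are empty, and the stun check is unconnected.
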(event Custom|OnAtkHitStart
  (bind _mesh (Variables|Character|GetMesh))
  (bind _outhit (Collision|SphereTraceByChannel (Transformation|GetSocketLocation _mesh "TrailStart") (Transformation|GetSocketLocation _mesh "TrailEnd") 5e+01 "TraceTypeQuery1" false 0 "ForDuration"))
  (if (Utilities|IsValid (Actor|GetComponentbyClass (.HitActor (Collision|BreakHitResult _outhit)) "/Game/Gridventure/Blueprints/Core/BPC_StatComponent.BPC_StatComponent_C"))
    (Default|TakeDmg (Actor|GetComponentbyClass (.HitActor (Collision|BreakHitResult _outhit)) "/Game/Gridventure/Blueprints/Core/BPC_StatComponent.BPC_StatComponent_C") self (.atk (Variables|/Game/Gridventure/Blueprints/Core/BPC_StatComponent.BPC_StatComponent_C|GetBaseStat (Variables|Default|GetBPC_StatComponent))) 1e+02)))

(event Custom|OnAtkHitEnd)

(event Custom|OnDamaged)

(event EventBeginPlay)

(event Collision|EventActorBeginOverlap
  (params (OtherActor :type Actor%20Object%20Reference)))

(event EventTick
  (params (DeltaSeconds :type Float%20%28single-precision%29)))

(event Game|Damage|EventAnyDamage
  (params (Damage :type Float%20%28single-precision%29) (DamageType :type Damage%20Type%20Object%20Reference) (InstigatedBy :type Controller%20Object%20Reference) (DamageCauser :type Actor%20Object%20Reference))
  ;[0.15 0.15 0.15 0.5] 데미지 전달
  (Default|TakeDmg (Variables|Default|GetBPC_StatComponent) self Damage 1e+02))

(fn ConstructionScript)