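; BP_BaseProjectile is a base projectile actor that damages Enemy-tagged actors and expires after a short default lifespan.
; Sphere overlaps apply damage credited to its owner and spawn a hit emitter, with a hit-actor list preventing repeat hits while piercing.
; Pierce and bounce counters decide when enemy or Environment contacts destroy it; this graph only counts bounces and does not redirect the projectile.
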(event OnComponentBeginOverlap(Sphere)
  (params (OverlappedComponent :type Primitive%20Component%20Object%20Reference) (OtherActor :type Actor%20Object%20Reference) (OtherComp :type Primitive%20Component%20Object%20Reference) (OtherBodyIndex :type Integer) (bFromSweep :type Boolean) (SweepResult :type Hit%20Result%20Structure%20%28by%20ref%29))
  (if (Actor|ActorHasTag OtherActor "Enemy")
    ;[0.15 0.15 0.15 0.5] 관통으로 중복 타격 방지
    (if (not (Utilities|Array|ContainsItem (Variables|Default|GetHitActors) OtherActor))
      (Utilities|FlowControl|Sequence
        (:then_0
          ;[0.15 0.15 0.15 0.5] 중복 방지 목록에 추가
          (Utilities|Array|Add (Variables|Default|GetHitActors) OtherActor))
        (:then_1
          ;[0.15 0.15 0.15 0.5] 데미지 적용
          (Game|Damage|ApplyDamage OtherActor (Variables|Default|GetDmg) (Game|GetInstigatorController (Variables|Default|GetOwnerRef)) (Variables|Default|GetOwnerRef) "/Script/Engine.DamageType"))
        (:then_2
          ;[0.15 0.15 0.15 0.5] Effect 생성
          (Effects|SpawnEmitteratLocation "/Game/TrailPack/Particles/Cascade/Magic/Hit/P_MagicHitSoft.P_MagicHitSoft" (Transformation|GetActorLocation)))
        (:then_3
          ;[0.15 0.15 0.15 0.5] 관통 체크
          (if (< (Variables|Default|GetCurPierce) (Variables|Default|GetPierceCnt))
            (bind _result (Math|Integer|IncrementInt (Variables|Default|GetCurPierce))
              (:%20%20
                (Variables|Default|SetCurPierce _result)))
            (else
              (Actor|DestroyActor) ; 삭제
            )))))
    (else
      ;[0.15 0.15 0.15 0.5] 팅기기 체크
      (if (Actor|ActorHasTag OtherActor "Environment")
        (if (> (Variables|Default|GetBounceCnt) 0)
          (Math|Integer|DecrementInt (Variables|Default|GetBounceCnt))
          (else
            (Actor|DestroyActor)))))))

(event EventBeginPlay
  ;[0.15 0.15 0.15 0.5] 기본 수명 2초
  (Actor|SetLifeSpan 2.0))

(fn ConstructionScript)