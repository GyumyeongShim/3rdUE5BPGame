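; Base monster character that chases the player, applies damage on capsule overlap with BP_BaseCharacter and drops an experience gem on death.
; Construction loads mesh, stats and hit montage from a hard-coded DT_MonsterData row, but BeginPlay overrides speed and hard-codes HP.
; A looping timer reissues AI MoveTo until within range.
; Hits trigger a montage, floating damage text and material flash; death enables ragdoll, plays a montage and sets a short lifespan.
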(event OnComponentBeginOverlap(Capsule)
  (params (OverlappedComponent :type Primitive%20Component%20Object%20Reference) (OtherActor :type Actor%20Object%20Reference) (OtherComp :type Primitive%20Component%20Object%20Reference) (OtherBodyIndex :type Integer) (bFromSweep :type Boolean) (SweepResult :type Hit%20Result%20Structure%20%28by%20ref%29))
  (if (Utilities|Enum|Equal(Enum) (Variables|Default|GetState) "NewEnumerator0")
    (bind _asbp_base_character (Utilities|Casting|CastToBP_BaseCharacter OtherActor))
    (Utilities|IsValid _asbp_base_character
      (:Is%20Valid
        (Game|Damage|ApplyDamage 0 1e+01 0 0)))))

(event Custom|PlayHitFlash
  ;[0.15 0.15 0.15 0.5] 피격시 붉은 외곽선
  (Rendering|Material|SetScalarParameterValue (Variables|Default|GetHitFlash) "FlashIntensity" 1.0 :!class /Script/Engine.MaterialInstanceDynamic)
  (Utilities|FlowControl|Delay 0.3)
  (Rendering|Material|SetScalarParameterValue (Variables|Default|GetHitFlash) "FlashIntensity" 0.0 :!class /Script/Engine.MaterialInstanceDynamic))

(event Custom|SetVIsibility
  (Rendering|SetVisibility (Variables|Default|GetWidget_DmgText) false false))

(event Custom|MoveToPlayer
  (bind _returnvalue (Game|GetPlayerCharacter 0))
  (bind _returnvalue_2 (Game|GetPlayerCharacter 0))
  (Utilities|IsValid _returnvalue_2
    (:Is%20Valid
      (if (> (Transformation|GetDistanceTo _returnvalue_2) 1.5e+02)
        (AI|AIMoveTo self (Transformation|GetActorLocation _returnvalue) _returnvalue 3e+01 false)
        (else
          (Components|Movement|StopMovementImmediately (Variables|Character|GetCharacterMovement)))))))

(event EventBeginPlay
  (Utilities|Time|SetTimerbyEvent (delegate Custom|MoveToPlayer) 0.5 true)
  (Variables|Default|SetCurHp 1e+02)
  (Variables|/Script/Engine.CharacterMovementComponent|SetMaxWalkSpeed (Variables|Character|GetCharacterMovement) 2e+02)
  (bind _returnvalue (Rendering|Material|CreateDynamicMaterialInstance (Variables|Character|GetMesh) 0 "/Game/Assets/Materials/Skeleton_Crossbowman_Material.Skeleton_Crossbowman_Material" "None" :!class /Script/Engine.PrimitiveComponent))
  (Utilities|IsValid _returnvalue
    (:Is%20Valid
      (Variables|Default|SetHitFlash _returnvalue)
      (bind _aswbp_dmg_text (Utilities|Casting|CastToWBP_DmgText (UserInterface|GetUserWidgetObject (Variables|Default|GetWidget_DmgText))))
      (Utilities|IsValid _aswbp_dmg_text
        (:Is%20Valid
          (EventDispatchers|BindEventtoOnFloatingDmgTxtAniFinished _aswbp_dmg_text (delegate Custom|SetVIsibility)))))))

(event Game|Damage|EventAnyDamage
  (params (Damage :type Float%20%28single-precision%29) (DamageType :type Damage%20Type%20Object%20Reference) (InstigatedBy :type Controller%20Object%20Reference) (DamageCauser :type Actor%20Object%20Reference))
  ;[0.15 0.15 0.15 0.5] 피격 처리
  (if (Utilities|Enum|Equal(Enum) (Variables|Default|GetState) "NewEnumerator0")
    (bind _output_get (Variables|Default|SetCurHp (- (Variables|Default|GetCurHp) Damage)))
    (CallFunction|PlayHitReaction)
    (Rendering|SetVisibility (Variables|Default|GetWidget_DmgText) true false)
    (bind _aswbp_dmg_text (Utilities|Casting|CastToWBP_DmgText (UserInterface|GetUserWidgetObject (Variables|Default|GetWidget_DmgText))))
    (Utilities|IsValid _aswbp_dmg_text
      (:Is%20Valid
        (Default|PlayFloatingDmgAni _aswbp_dmg_text Damage)
        (CallFunction|PlayHitFlash)
        (if (<= _output_get 0.0)
          (CallFunction|Dead))))))

(fn ConstructionScript
  (bind _returnvalue (Utilities|GetDataTableRow "/Game/Gridventure/Blueprints/Data/DT_MonsterData.DT_MonsterData" "Skeleton_CB")
    (:then
      (Utilities|FlowControl|Sequence
        (:then_0
          (bind _output_get (Variables|Default|SetBaseStat (.basestat _returnvalue)))
          (Variables|/Script/Engine.CharacterMovementComponent|SetMaxWalkSpeed (Variables|Character|GetCharacterMovement) (.spd _output_get)))
        (:then_1
          (Components|SkeletalMesh|SetSkeletalMeshAsset (Variables|Character|GetMesh) (.monstermesh _returnvalue)))
        (:then_2
          (Variables|Default|SetAnimBP (.animbp _returnvalue))
          (Variables|Default|SetHitMontage (.hitmontage _returnvalue)))))))

(fn PlayHitReaction
  (Animation|PlayAnimMontage (Variables|Default|GetHitMontage) 1.0 "None"))

(fn Dead
  (bind _mesh (Variables|Character|GetMesh))
  (bind _capsulecomponent (Variables|Collision|GetCapsuleComponent))
  (Utilities|FlowControl|Sequence
    (:then_0
      (Components|Movement|StopMovementImmediately (Variables|Character|GetCharacterMovement)) ; 이동 제거
      (Collision|SetCollisionEnabled _capsulecomponent "QueryAndPhysics") ; 바닥을 지탱할 메쉬의 설정
      (Collision|SetCollisionResponsetoAllChannels _capsulecomponent "ECR_Ignore")
      (Collision|SetCollisionResponsetoChannel _capsulecomponent "ECC_WorldDynamic" "ECR_Block")
      (Collision|SetCollisionResponsetoChannel _capsulecomponent "ECC_WorldStatic" "ECR_Block")
      ;[0.15 0.15 0.15 0.5] ragdoll을 사용한 물리 시뮬레이션
      (Physics|SetSimulatePhysics _mesh true)
      (Collision|SetCollisionProfileName _mesh "Ragdoll" true :!class /Script/Engine.PrimitiveComponent)
      (Class|PrimitiveComponent|SetAllPhysicsLinearVelocity _mesh "0, 0, 0" false))
    (:then_1
      ;[0.15 0.15 0.15 0.5] 사망 애니메이션
      (Animation|PlayAnimMontage (Variables|Default|GetDeadMontage) 1.0 "None")
      (Variables|Default|SetState "NewEnumerator1"))
    (:then_2
      (CallFunction|SpawnExpGem))
    (:then_3
      ;[0.15 0.15 0.15 0.5] 삭제 처리
      (Actor|SetLifeSpan 2.0))))

(fn SpawnExpGem
  (Game|SpawnActorfromClass "/Game/Gridventure/Blueprints/Actor/BP_ExpGem.BP_ExpGem_C" (Math|Conversions|ToTransform(Vector) (+ (Transformation|GetActorLocation) "0.000000,0.000000,50.000000")) "AlwaysSpawn" "MultiplyWithRoot" self 1e+01 0))