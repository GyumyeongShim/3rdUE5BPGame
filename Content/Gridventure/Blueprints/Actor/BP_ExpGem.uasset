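; Experience gem pickup that drops to the floor on spawn, then homes in on the player and grants EXP when absorbed.
; A timeline lerps the drop, then a looping timer checks player range and starts an absorb timeline that uses VInterpTo with curve-driven speed.
; On contact distance it destroys itself and adds fixed EXP through BPC_StatComponent.
; An older chase using ExpValue and a Niagara impact remains disconnected.
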(event Custom|CheckDist
  (if (< (Transformation|GetDistanceTo (Game|GetPlayerCharacter 0)) 7e+02)
    (if (Variables|Default|GetIsTracking)
      (CallFunction|ChasingAbsorb)
      (else
        (Variables|Default|SetIsTracking true)))))

(event Custom|Chasing%20Absorb
  ;[0.15 0.15 0.15 0.5] 추적 흡수
  (bind _speedcurve (Timeline|TM_Absorb PlayFromStart)
    (:Update
      (Transformation|SetActorLocation (Math|Interpolation|VInterpTo (Transformation|GetActorLocation) (Transformation|GetActorLocation (Game|GetPlayerCharacter 0)) (Utilities|Time|GetWorldDeltaSeconds) _speedcurve) false false)
      (if (< (Transformation|GetDistanceTo (Game|GetPlayerCharacter 0)) 3e+01)
        (Actor|DestroyActor)
        (Default|AddExp (Actor|GetComponentbyClass (Game|GetPlayerCharacter 0) "/Game/Gridventure/Blueprints/Core/BPC_StatComponent.BPC_StatComponent_C") 1e+01)
        (else
          (Variables|Default|SetIsTracking false))))))

(event EventBeginPlay
  ;[0.15 0.15 0.15 0.5] Item Drop
  (|InitValue)
  (bind _tm_drop (Timeline|DropToFloor PlayFromStart)
    (:Update
      (Transformation|SetActorLocation (Math|Vector|Lerp(Vector) (Variables|Default|GetStartLocation) (Variables|Default|GetTargetLocation) _tm_drop) false false))
    (:Finished
      (Utilities|Time|SetTimerbyEvent (delegate Custom|CheckDist) 0.3 true))))

(event EventTick
  (params (DeltaSeconds :type Float%20%28single-precision%29)))

(fn ConstructionScript)