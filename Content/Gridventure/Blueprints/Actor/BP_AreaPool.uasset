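; BP_AreaPool is a temporary damage-over-time area actor that harms actors within its radius while sparing the first player character.
; On BeginPlay it sizes the sphere collision and Niagara effect from Radius, sets its lifespan from Duration and starts a short looping timer.
; Each tick of that timer applies radial damage at the pool's location using Dot as base damage, ignoring itself and that player.
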(event Custom|ApplyDot
  (Game|Damage|ApplyRadialDamage (Variables|Default|GetDot) (Transformation|GetActorLocation) (Variables|Default|GetRadius) 0 (Utilities|Array|MakeArray (Game|GetPlayerCharacter 0) self) 0 0 false "ECC_Visibility"))

(event EventBeginPlay
  (Components|Sphere|SetSphereRadius (Variables|Default|GetSphereCollision) (Variables|Default|GetRadius) true)
  (Niagara|SetNiagaraVariable(Float) (Variables|Default|GetNiagara) "User.Radius" (Variables|Default|GetRadius))
  (Actor|SetLifeSpan (Variables|Default|GetDuration))
  (Utilities|Time|SetTimerbyEvent (delegate Custom|ApplyDot) 0.3 true))

(fn ConstructionScript)