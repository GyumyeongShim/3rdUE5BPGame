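; BP_MonsterSpawner is an actor that periodically spawns BP_BaseMonster around the player.
; BeginPlay starts a looping timer at SpawnRate, and each tick spawns a monster, adjusting for collision but always spawning.
; GetSpawnLocation offsets player controller 0's location by a random horizontal direction and a distance between MinRadius and MaxRadius, with Z fixed at zero.
; It also draws a red debug sphere on each call.
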(event Custom|SpawnEnemy
  (bind _pos (CallFunction|GetSpawnLocation))
  (Game|SpawnActorfromClass "/Game/Gridventure/Blueprints/Actor/BP_BaseMonster.BP_BaseMonster_C" (Math|Conversions|ToTransform(Vector) _pos) "AdjustIfPossibleButAlwaysSpawn" "MultiplyWithRoot" 0 0))

(event EventBeginPlay
  (Utilities|Time|SetTimerbyEvent (delegate Custom|SpawnEnemy) (Variables|Default|GetSpawnRate) true))

(fn ConstructionScript)

(fn GetSpawnLocation
  (bind _returnvalue (Game|GetPlayerController 0))
  (bind _returnvalue_2 (Math|Random|RandomUnitVector))
  (bind _minradius (Variables|Default|GetMinRadius))
  (bind _maxradius (Variables|Default|GetMaxRadius))
  (bind _returnvalue_3 (Transformation|GetActorLocation _returnvalue))
  (bind _returnvalue_4 (Math|Random|RandomFloatinRange _minradius _maxradius))
  (bind _returnvalue_5 (Math|Vector|MakeVector (.x _returnvalue_2) (.y _returnvalue_2) 0.0))
  (bind _returnvalue_6 (Math|Vector|Normalize _returnvalue_5 0.0))
  (bind _returnvalue_7 (* _returnvalue_6 _returnvalue_4))
  (bind _returnvalue_8 (+ _returnvalue_3 _returnvalue_7))
  (bind (_x _y) (Math|Vector|BreakVector _returnvalue_8))
  (Rendering|Debug|DrawDebugSphere "0, 0, 0" 1e+02 12 "(R=1.000000,G=0.000000,B=0.000000,A=1.000000)" 0.0)
  (return (Math|Vector|MakeVector _x _y 0.0)))