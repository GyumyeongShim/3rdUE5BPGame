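; Inventory utility function library with GetAdjacentIndicesByShape, evidently meant to find grid cells surrounding a shape placed at an origin index.
; It converts shape offsets into unique flattened indices, then scans each one's 3x3 neighborhood.
; As wired, it keeps candidates whose occupied and in-bounds states match, so free in-bounds neighbors are excluded.
; GridHeight bounds Y times width in the first pass but Y alone in the second.
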(fn GetAdjacentIndicesbyShape
  (params (OriginIdx :type Integer) (OccupiedCells :type Array%20of%20Vector%202D%20Structures) (GridWidth :type Integer) (GridHeight :type Integer))
  (Utilities|FlowControl|Sequence
    (:then_0
      (for _array_element OccupiedCells
        (if (and (and (>= (+ (.x _array_element) (Math|Integer|%(Integer) OriginIdx GridWidth)) 0.0) (< (+ (.x _array_element) (Math|Integer|%(Integer) OriginIdx GridWidth)) GridWidth)) (and (>= (+ (.y _array_element) (/ OriginIdx GridWidth)) 0.0) (< (* (+ (.y _array_element) (/ OriginIdx GridWidth)) GridWidth) GridHeight)))
          (Utilities|Array|AddUnique (LocalVariables|GetActualOccupiedIndices) (Math|Float|Truncate (+ (+ (.x _array_element) (Math|Integer|%(Integer) OriginIdx GridWidth)) (* (+ (.y _array_element) (/ OriginIdx GridWidth)) GridWidth)))))))
    (:then_1
      (for _array_element_2 (LocalVariables|GetActualOccupiedIndices)
        ;[0.15 0.15 0.15 0.5] X = (element%Width)
        (for _index (range -1 1)
          ;[0.15 0.15 0.15 0.5] Y = (element / Width) + idx
          (for _index_2 (range -1 1)
            (if (not (!= (Utilities|Array|ContainsItem (LocalVariables|GetActualOccupiedIndices) (+ (* (+ (/ _array_element_2 GridWidth) _index_2) GridWidth) (+ _index (Math|Integer|%(Integer) _array_element_2 GridWidth)))) (and (and (>= (+ _index (Math|Integer|%(Integer) _array_element_2 GridWidth)) 0) (< (+ _index (Math|Integer|%(Integer) _array_element_2 GridWidth)) GridWidth)) (and (>= (+ (/ _array_element_2 GridWidth) _index_2) 0) (< (+ (/ _array_element_2 GridWidth) _index_2) GridHeight)))))
              (Utilities|Array|AddUnique (LocalVariables|GetOutAdjacentIndice) (+ (* (+ (/ _array_element_2 GridWidth) _index_2) GridWidth) (+ _index (Math|Integer|%(Integer) _array_element_2 GridWidth))))))))
      (return (LocalVariables|GetOutAdjacentIndice)))))