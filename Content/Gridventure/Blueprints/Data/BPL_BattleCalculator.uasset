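; Blueprint function library of battle formulas for Gridventure, covering final damage, hit rolls and critical rolls.
; Damage scales attack by a percentage power, applies diminishing defense mitigation, adds a small random variance and has a minimum floor.
; Hit and critical checks are independent percentage rolls against accuracy minus evasion and crit chance minus resistance.
; Hit chance keeps a small guaranteed minimum, while crit chance is floored at zero.
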(fn GetFinalDmg
  (params (Atk :type Float%20%28double-precision%29) (Def :type Float%20%28double-precision%29) (Power :type Float%20%28double-precision%29))
  (return (Math|Float|Max(Float) 1.0 (* (* (* Atk (* Power 0.01)) (/ 1e+02 (+ Def 1e+02))) (Math|Random|RandomFloatinRange 0.9 1.1)))))

(fn CalcHitChance
  (params (Acc :type Float%20%28double-precision%29) (Evasion :type Float%20%28double-precision%29))
  (return (<= (Math|Random|RandomFloatinRange 0.0 1e+02) (Math|Float|Max(Float) (- Acc Evasion) 5.0))))

(fn CalcCri
  (params (CriChance :type Float%20%28double-precision%29) (CriResist :type Float%20%28double-precision%29))
  (return (<= (Math|Random|RandomFloatinRange 0.0 1e+02) (Math|Float|Max(Float) (- CriChance CriResist) 0.0))))